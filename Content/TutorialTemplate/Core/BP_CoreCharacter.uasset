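; Base player character for the tutorial template that handles movement, aiming, jumping and sprinting from keyboard/mouse and gamepad inputs.
; Paired input events feed shared helpers, with movement following control yaw only.
; A LockInput macro gates movement, aim, jump and sprint start on a boolean, while releases always go through.
; Sprint swaps walk speed with the default cached at BeginPlay, held on the standard binding but toggled on gamepad.
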(event `self.ReceiveBeginPlay`
  (set `self.DefaultSpeed` (`CharacterMovementComponent.MaxWalkSpeed` (`self.CharacterMovement`))))

(event `InputAction|Jump` :overrideparent false
  (params (Key :type "Key Structure"))
  (:`Pressed`
    (`self.LockInput` :!label _label
      (:`false`
        (`self.Jump`))))
  (:`Released`
    (`self.StopJumping` :!label _label_2)))

(event `InputAction|GP_Jump`
  (params (Key :type "Key Structure"))
  (:`Pressed`
    (goto _label))
  (:`Released`
    (goto _label_2)))

(event `InputAxis|MoveForward`
  (params (AxisValue :type "Float (single-precision)"))
  (`self.AddMovementForward` AxisValue))

(event `InputAxis|GP_MoveForward`
  (params (AxisValue :type "Float (single-precision)"))
  (`self.AddMovementForward` AxisValue))

(event `InputAction|Sprint`
  (params (Key :type "Key Structure"))
  (:`Pressed`
    (`self.LockInput` :!label _label_3
      (:`false`
        (set `CharacterMovementComponent.MaxWalkSpeed` (`self.SprintSpeed`) (`self.CharacterMovement`)))))
  (:`Released`
    (set `CharacterMovementComponent.MaxWalkSpeed` (`self.DefaultSpeed`) (`self.CharacterMovement`) :!label _label_4)))

(event `InputAxis|MoveBackward`
  (params (AxisValue :type "Float (single-precision)"))
  (`self.AddMovementForward` AxisValue))

(event `InputAxis|GP_MoveBackward`
  (params (AxisValue :type "Float (single-precision)"))
  (`self.AddMovementForward` AxisValue))

(event `InputAction|GP_Sprint`
  (params (Key :type "Key Structure"))
  (:`Pressed`
    (`/Engine/EditorBlueprintResources/StandardMacros.FlipFlop`
      (:`A`
        (goto _label_3))
      (:`B`
        (goto _label_4)))))

(event `InputAxis|StrafeLeft`
  (params (AxisValue :type "Float (single-precision)"))
  (`self.AddMovementRight` AxisValue))

(event `InputAxis|GP_StrafeLeft`
  (params (AxisValue :type "Float (single-precision)"))
  (`self.AddMovementRight` AxisValue))

(event `InputAxis|GP_StrafeRight`
  (params (AxisValue :type "Float (single-precision)"))
  (`self.AddMovementRight` AxisValue))

(event `InputAxis|StrafeRight`
  (params (AxisValue :type "Float (single-precision)"))
  (`self.AddMovementRight` AxisValue))

(event `InputAxis|XAim`
  (params (AxisValue :type "Float (single-precision)"))
  (`self.AddYawAim` AxisValue))

(event `InputAxis|GP_XAim`
  (params (AxisValue :type "Float (single-precision)"))
  (`self.AddYawAim` AxisValue))

(event `InputAxis|YAim`
  (params (AxisValue :type "Float (single-precision)"))
  (`self.AddPitchAim` AxisValue))

(event `InputAxis|GP_YAim`
  (params (AxisValue :type "Float (single-precision)"))
  (`self.AddPitchAim` AxisValue))

(fn `AddMovementForward`
  (params (ScaleValue :type "Float (double-precision)"))
  (bind (_returnvalue_roll _returnvalue_pitch _returnvalue_yaw) (`KismetMathLibrary.BreakRotator` (`self.GetControlRotation`)))
  (`self.LockInput`
    (:`false`
      (`self.AddMovementInput` self (`KismetMathLibrary.GetForwardVector` (`KismetMathLibrary.MakeRotator` 0.0 0.0 _returnvalue_yaw)) ScaleValue false))))

(fn `AddMovementRight`
  (params (ScaleValue :type "Float (double-precision)"))
  (bind (_returnvalue_roll _returnvalue_pitch _returnvalue_yaw) (`KismetMathLibrary.BreakRotator` (`self.GetControlRotation`)))
  (`self.LockInput`
    (:`false`
      (`self.AddMovementInput` self (`KismetMathLibrary.GetRightVector` (`KismetMathLibrary.MakeRotator` 0.0 0.0 _returnvalue_yaw)) ScaleValue false))))

(fn `AddPitchAim`
  (params (Val :type "Float (double-precision)"))
  (`self.LockInput`
    (:`false`
      (`self.AddControllerPitchInput` Val))))

(fn `AddYawAim`
  (params (Val :type "Float (double-precision)"))
  (`self.LockInput`
    (:`false`
      (`self.AddControllerYawInput` Val))))

(fn `UserConstructionScript`)